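; Clickable chair actor that shows a WB_ChairsUI widget and provides transform data for seating.
; Clicking the hovered mesh hides the widget of the player controller's previous chair, shows this one, passes itself to the UI and registers as CurrentChair.
; CalcTransData derives a seat location and rotation from height, forward offset and a yaw offset on the mesh's rotation.
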(event `self.ReceiveTick`
  (params (DeltaSeconds :type "Float (single-precision)")))

(event `self.ReceiveBeginPlay`
  (`self.ShowHideWidget` true))

(event `self.ItemMesh.OnBeginCursorOver`
  (params (TouchedComponent :type "PrimitiveComponent Object Reference"))
  (set `self.bHover` true)
  (`KismetSystemLibrary.PrintString` "11111"))

(event `self.ItemMesh.OnEndCursorOver`
  (params (TouchedComponent :type "PrimitiveComponent Object Reference"))
  (set `self.bHover` false)
  (`KismetSystemLibrary.PrintString` "2222"))

(event `self.ItemMesh.OnClicked`
  (params (TouchedComponent :type "PrimitiveComponent Object Reference") (ButtonPressed :type "Key Structure"))
  (if (`self.bHover`)
    (`self.Check Chair and Show Widget`) ; 检查当前座椅和显示UI
  ))

(fn `Calc Trans Data`
  (params (InAngleOffset :type "Float (double-precision)" :default 90.0) (ChairHeight :type "Float (double-precision)" :default 100.0))
  (returns (NewLocation :type "Vector Structure") (NewRotation :type "Rotator Structure"))
  (bind _returnvalue (`self.RotOffset` InAngleOffset))
  (bind _setoffsetval (`self.SetOffsetVal`))
  (return (+ (`self.K2_GetActorLocation`) (`KismetMathLibrary.MakeVector` 0.0 0.0 ChairHeight) (* (`KismetMathLibrary.GetForwardVector` _returnvalue) (`KismetMathLibrary.MakeVector` _setoffsetval _setoffsetval))) _returnvalue))

(fn `Check Chair and Show Widget`
  (locals (CurrentPlayerController :type "/Game/FangChan/Blueprint/System/BP_PlayerConotroller Object Reference"))
  (bind (_bisvalid _asbp_player_conotroller) (`/Game/FangChan/Blueprint/System/BP_FunctionLib.GetCurrentPlayerController`))
  (bind (_isvaild _outwb_chairs_ui) (`self.GetOwenrWidget`))
  (bind _currentchair (`/Game/FangChan/Blueprint/System/BP_PlayerConotroller.CurrentChair` (`local.CurrentPlayerController`)))
  (if _bisvalid
    (set `local.CurrentPlayerController` _asbp_player_conotroller)
    (`/Engine/EditorBlueprintResources/StandardMacros.IsValid` _currentchair
      (:`Is Valid`
        (if (!= _currentchair self)
          (`self.ShowHideWidget` _currentchair true) ; 隐藏之前的
        ))
      (:`Is Not Valid`
        _))
    ;[1 1 1] 开启当前的
    (`self.ShowHideWidget` false)
    (if _isvaild
      (`/Game/FangChan/Blueprint/UI/WB_ChairsUI.GetInfo` _outwb_chairs_ui self)
      (set `/Game/FangChan/Blueprint/System/BP_PlayerConotroller.CurrentChair` self (`local.CurrentPlayerController`)))))

(fn `GetOwenrWidget`
  (returns (IsVaild :type Boolean) (`OutWB Chairs UI` :type "/Game/FangChan/Blueprint/UI/WB_ChairsUI Object Reference"))
  (bind _aswb_chairs_ui (cast `/Game/FangChan/Blueprint/UI/WB_ChairsUI` (`WidgetComponent.GetWidget` (`self.ButtonWidget`)))
    (:`then`
      (return true _aswb_chairs_ui))
    (:`CastFailed`
      (return false null))))

(fn `RotOffset`
  (params (InAngle :type "Float (double-precision)" :default 90.0))
  (returns (ReturnValue :type "Rotator Structure"))
  (bind (_returnvalue_roll _returnvalue_pitch _returnvalue_yaw) (`KismetMathLibrary.BreakRotator` (`SceneComponent.K2_GetComponentRotation` (`self.ItemMesh`))))
  (return (`KismetMathLibrary.MakeRotator` _returnvalue_roll _returnvalue_pitch (+ _returnvalue_yaw InAngle))))

(fn `ShowHideWidget`
  (params (bHidden :type Boolean))
  (`SceneComponent.SetHiddenInGame` (`self.ButtonWidget`) bHidden false))

(fn `UserConstructionScript`)