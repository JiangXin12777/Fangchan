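; BP_Video is a proximity-triggered video actor that plays its MediaSource when BP_ThirdPersonCharacter enters its Box or Capsule volume.
; Both volumes feed a shared overlap counter, Index, opening the source when it rises to 0 and closing it when it falls to -1.
; On BeginPlay and after that close, Reset briefly opens then closes the source, and BeginPlay also binds MediaSound to the MediaPlayer after a delay.
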(event `self.ReceiveBeginPlay`
  (`self.Reset`)
  (`KismetSystemLibrary.Delay` 1.0)
  (`MediaSoundComponent.SetMediaPlayer` (`self.MediaSound`) (`self.MediaPlayer`)))

(event `self.Box.OnComponentBeginOverlap`
  (params (OverlappedComponent :type "PrimitiveComponent Object Reference") (OtherActor :type "Actor Object Reference") (OtherComp :type "PrimitiveComponent Object Reference") (OtherBodyIndex :type Integer) (bFromSweep :type Boolean) (SweepResult :type "HitResult Structure (by ref)"))
  (`self.CharacterBeginOverlap` OtherActor))

(event `self.Box.OnComponentEndOverlap`
  (params (OverlappedComponent :type "PrimitiveComponent Object Reference") (OtherActor :type "Actor Object Reference") (OtherComp :type "PrimitiveComponent Object Reference") (OtherBodyIndex :type Integer))
  (`self.CharacterEndOverlap` OtherActor))

(event `self.Capsule.OnComponentBeginOverlap`
  (params (OverlappedComponent :type "PrimitiveComponent Object Reference") (OtherActor :type "Actor Object Reference") (OtherComp :type "PrimitiveComponent Object Reference") (OtherBodyIndex :type Integer) (bFromSweep :type Boolean) (SweepResult :type "HitResult Structure (by ref)"))
  (`self.CharacterBeginOverlap` OtherActor))

(event `self.Capsule.OnComponentEndOverlap`
  (params (OverlappedComponent :type "PrimitiveComponent Object Reference") (OtherActor :type "Actor Object Reference") (OtherComp :type "PrimitiveComponent Object Reference") (OtherBodyIndex :type Integer))
  (`self.CharacterEndOverlap` OtherActor))

(event `Reset`
  (bind _mediaplayer (`self.MediaPlayer`))
  (bind _media_source (`self.Media Source`))
  (if (and (`KismetSystemLibrary.IsValid` _mediaplayer) (`KismetSystemLibrary.IsValid` _media_source))
    (`MediaPlayer.OpenSource` _mediaplayer _media_source)
    (`KismetSystemLibrary.Delay` 0.5)
    (`MediaPlayer.Close` _mediaplayer)))

(fn `CharacterBeginOverlap`
  (params (InCActor :type "Actor Object Reference"))
  (bind _mediaplayer (`self.MediaPlayer`))
  (bind _media_source (`self.Media Source`))
  (bind _asbp_third_person_character (cast `/Game/ThirdPerson/Blueprints/BP_ThirdPersonCharacter` InCActor))
  (`|ExecutionSequence`
    (:`then_0`
      (`/Engine/EditorBlueprintResources/StandardMacros.IsValid` _asbp_third_person_character
        (:`Is Valid`
          (`/Engine/EditorBlueprintResources/StandardMacros.IncrementInt` (`self.Index`)))))
    (:`then_1`
      (if (== (`self.Index`) 0)
        (if (and (`KismetSystemLibrary.IsValid` _mediaplayer) (`KismetSystemLibrary.IsValid` _media_source))
          (`MediaPlayer.OpenSource` _mediaplayer _media_source))))))

(fn `CharacterEndOverlap`
  (params (InActor :type "Actor Object Reference"))
  (bind _mediaplayer (`self.MediaPlayer`))
  (bind _asbp_third_person_character (cast `/Game/ThirdPerson/Blueprints/BP_ThirdPersonCharacter` InActor))
  (`|ExecutionSequence`
    (:`then_0`
      (`/Engine/EditorBlueprintResources/StandardMacros.IsValid` _asbp_third_person_character
        (:`Is Valid`
          (`/Engine/EditorBlueprintResources/StandardMacros.DecrementInt` (`self.Index`)))))
    (:`then_1`
      (if (== (`self.Index`) -1)
        (`/Engine/EditorBlueprintResources/StandardMacros.IsValid` _mediaplayer
          (:`Is Valid`
            (`MediaPlayer.Close` _mediaplayer)
            (`self.Reset`)))))))

(fn `UserConstructionScript`)