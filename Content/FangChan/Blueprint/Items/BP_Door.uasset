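; BP_Door is a clickable door that opens and closes with a material dissolve effect.
; Cursor hover on Box sets CanInteractive and shows a WB_Label prompt reading open or close (开门/关门) while no animation runs.
; Clicking plays or reverses DoorOpenTimeline, which drives the DissolveAmount material parameter.
; The door is hidden without collision once opened, and is restored before the closing animation starts.
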(event `self.ReceiveBeginPlay`
  (`self.SetDoorStatus` true))

(event `self.Box.OnBeginCursorOver`
  (params (TouchedComponent :type "PrimitiveComponent Object Reference"))
  (set `self.bCanInteractive` true)
  (`KismetSystemLibrary.PrintString` "can Interactive")
  (`self.Set Widget Status`))

(event `self.Box.OnEndCursorOver`
  (params (TouchedComponent :type "PrimitiveComponent Object Reference"))
  (set `self.bCanInteractive` false)
  (`KismetSystemLibrary.PrintString` "cant Interactive" true true (struct :`R` 1.0 :`B` 0.11367 :`A` 1.0))
  (`self.Set Widget Status`))

(event `self.Box.OnClicked`
  (params (TouchedComponent :type "PrimitiveComponent Object Reference") (ButtonPressed :type "Key Structure"))
  ;[1 1 1] j交互逻辑
  (if (`self.bCanInteractive`)
    (if (`self.bDoorOpened`)
      (`self.SetDoorStatus` true))
    (`SceneComponent.SetVisibility` (`self.Label`) false false)
    (set `self.bAnimFinished` false)
    (if (not (`self.bDoorOpened`))
      (bind (_direction _actionline) (`Timeline|DoorOpenTimeline` :!label _label)
        (:`Update`
          (`KismetSystemLibrary.PrintString` (`KismetStringLibrary.Conv_DoubleToString` _actionline))
          (`MeshComponent.SetScalarParameterValueOnMaterials` (`self.Door`) "DissolveAmount" _actionline))
        (:`Finished`
          (set `self.bDoorOpened` (not (`self.bDoorOpened`)))
          (set `self.bAnimFinished` true)
          (if (`self.bDoorOpened`)
            (`self.SetDoorStatus` false))))
      (else
        (goto _label :!via `Reverse`)))))

(fn `GetWidget`
  (returns (IsValid :type Boolean) (`AsWB Label` :type "/Game/FangChan/Blueprint/UI/WB_Label Object Reference"))
  (bind _aswb_label (cast `/Game/FangChan/Blueprint/UI/WB_Label` (`WidgetComponent.GetWidget` (`self.Label`)))
    (:`then`
      (return true _aswb_label))
    (:`CastFailed`
      (return false null))))

(fn `Set Widget Status`
  (locals (Widget :type "/Game/FangChan/Blueprint/UI/WB_Label Object Reference"))
  (bind (_isvalid _aswb_label) (`self.GetWidget`))
  (bind _label (`self.Label`))
  (if (and (`self.bCanInteractive`) (`self.bAnimFinished`))
    (`SceneComponent.SetVisibility` _label true false)
    (if _isvalid
      (if (`self.bDoorOpened`)
        (`/Game/FangChan/Blueprint/UI/WB_Label.SetTextInfo` _aswb_label "关门")
        (else
          (`/Game/FangChan/Blueprint/UI/WB_Label.SetTextInfo` _aswb_label "开门"))))
    (else
      (`SceneComponent.SetVisibility` _label false false))))

(fn `SetDoorStatus`
  (params (bShow :type Boolean))
  (bind _door (`self.Door`))
  (`SceneComponent.SetHiddenInGame` (`self.Door`) (not bShow) false)
  (if bShow
    (`SceneComponent.SetHiddenInGame` _door false false)
    (`PrimitiveComponent.SetCollisionEnabled` (`self.Door`) "QueryAndPhysics")
    (else
      (`SceneComponent.SetHiddenInGame` _door true false)
      (`PrimitiveComponent.SetCollisionEnabled` (`self.Door`) "NoCollision"))))

(fn `UserConstructionScript`)